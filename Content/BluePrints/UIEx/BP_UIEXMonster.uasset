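; Pirate monster character for a UI example, with a floating HP bar, damage numbers and hover cursor.
; BeginPlay spawns the HP bar, which Tick keeps at its anchor and turned toward the camera.
; Any capsule overlap spawns camera-facing damage text, clears the behavior tree, launches the monster away from the camera and flashes hit materials three times.
; Nodes restoring AI and knockback state are disconnected.
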(event `LookAtPlayer`
  (bind _returnvalue (- (`self.K2_GetActorLocation` (`GameplayStatics.GetPlayerCameraManager` 0)) (`self.K2_GetActorLocation`)))
  (set `self.DistancePlayer` (`KismetMathLibrary.VSize` _returnvalue))
  (set `self.DirtoPlayer` (`KismetMathLibrary.Normal` _returnvalue)))

(event `self.ReceiveBeginPlay`
  (bind _returnvalue (`|SpawnActorFromClass` "/Game/BluePrints/UIEx/MonsterHPBar.MonsterHPBar_C" (`KismetMathLibrary.MakeTransform` (`SceneComponent.K2_GetComponentLocation` (`self.HPBarPos`))) "Undefined" "OverrideRootScale" null null))
  (set `self.CurHPBar` _returnvalue))

(event `self.ReceiveTick`
  (params (DeltaSeconds :type "Float (single-precision)"))
  (`self.LookAtPlayer`)
  (`/Game/BluePrints/UIEx/MonsterHPBar.Update Location` (`self.CurHPBar`) (`SceneComponent.K2_GetComponentLocation` (`self.HPBarPos`)))
  (`/Game/BluePrints/UIEx/MonsterHPBar.Update Rocation` (`self.CurHPBar`) (`KismetMathLibrary.FindLookAtRotation` (`self.K2_GetActorLocation`) (`self.K2_GetActorLocation` (`GameplayStatics.GetPlayerCameraManager` 0)))))

(event `self.CapsuleComponent.OnComponentBeginOverlap`
  (params (OverlappedComponent :type "PrimitiveComponent Object Reference") (OtherActor :type "Actor Object Reference") (OtherComp :type "PrimitiveComponent Object Reference") (OtherBodyIndex :type Integer) (bFromSweep :type Boolean) (SweepResult :type "HitResult Structure (by ref)"))
  (`self.DamageText`)
  (set `self.BehaviorTree` null)
  (set `self.IsKnockBack` true)
  (if true
    (`self.LaunchCharacter` (* (`self.DirtoPlayer`) (-600.0 -600.0 800.0)))
    (`self.SetMaterialHit`)
    (`KismetSystemLibrary.Delay` 0.09)
    (`self.Set MaterialRevert`)
    (`KismetSystemLibrary.Delay` 0.09)
    (`self.SetMaterialHit`)
    (`KismetSystemLibrary.Delay` 0.09)
    (`self.Set MaterialRevert`)
    (`KismetSystemLibrary.Delay` 0.09)
    (`self.SetMaterialHit`)
    (`KismetSystemLibrary.Delay` 0.09)
    (`self.Set MaterialRevert`)))

(event `self.CapsuleComponent.OnBeginCursorOver`
  (params (TouchedComponent :type "PrimitiveComponent Object Reference"))
  (set `PlayerController.CurrentMouseCursor` "Hand" (`GameplayStatics.GetPlayerController` 0)))

(event `DamageText`
  (bind _returnvalue (`|SpawnActorFromClass` "/Game/BluePrints/UIEx/BP_DamageText.BP_DamageText_C" (`KismetMathLibrary.MakeTransform` (+ (`SceneComponent.K2_GetComponentLocation` (`self.DamageTextPos`)) (-0.0 0.0 0.0))) "Undefined" "OverrideRootScale" null null))
  (set `self.CurDamageText` _returnvalue)
  (`/Game/BluePrints/UIEx/BP_DamageText.SetDamageText` _returnvalue (`self.Damage`))
  (`/Game/BluePrints/UIEx/BP_DamageText.UpdateRotation` (`self.CurDamageText`) (`KismetMathLibrary.FindLookAtRotation` (`self.K2_GetActorLocation`) (`self.K2_GetActorLocation` (`GameplayStatics.GetPlayerCameraManager` 0)))))

(event `self.CapsuleComponent.OnEndCursorOver`
  (params (TouchedComponent :type "PrimitiveComponent Object Reference"))
  (set `PlayerController.CurrentMouseCursor` "Default" (`GameplayStatics.GetPlayerController` 0)))

(event `self.CapsuleComponent.OnClicked`
  (params (TouchedComponent :type "PrimitiveComponent Object Reference") (ButtonPressed :type "Key Structure")))

(fn `Set MaterialRevert`
  (bind _mesh (`self.Mesh`))
  (`PrimitiveComponent.SetMaterial` _mesh 0 "/Game/Pirate/Materials/M_Pirate_Cloth.M_Pirate_Cloth")
  (`PrimitiveComponent.SetMaterial` _mesh 1 "/Game/Pirate/Materials/M_Pirate_Body_1.M_Pirate_Body_1")
  (`PrimitiveComponent.SetMaterial` _mesh 2 "/Game/Pirate/Materials/M_Pirate_Hair_1.M_Pirate_Hair_1")
  (`PrimitiveComponent.SetMaterial` _mesh 3 "/Game/Pirate/Materials/M_Pirate_Details_Weapon.M_Pirate_Details_Weapon")
  (`PrimitiveComponent.SetMaterial` (`self.StaticMesh`) 0 "/Game/Resources/InfinityBladeWeapons/Weapons/Blade/Swords/Blade_BlackKnight/M_Blade_BlackKnight.M_Blade_BlackKnight"))

(fn `SetMaterialHit`
  (bind _mesh (`self.Mesh`))
  (`PrimitiveComponent.SetMaterial` _mesh 0 "/Game/Pirate/Materials/M_PirateHit_Inst.M_PirateHit_Inst")
  (`PrimitiveComponent.SetMaterial` _mesh 1 "/Game/Pirate/Materials/M_PirateHit_Inst.M_PirateHit_Inst")
  (`PrimitiveComponent.SetMaterial` _mesh 2 "/Game/Pirate/Materials/M_PirateHit.M_PirateHit")
  (`PrimitiveComponent.SetMaterial` _mesh 3 "/Game/Pirate/Materials/M_PirateHit.M_PirateHit")
  (`PrimitiveComponent.SetMaterial` (`self.StaticMesh`) 0 "/Game/Pirate/Materials/M_PirateHit.M_PirateHit"))

(fn `UserConstructionScript`)