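; Floating damage number actor that shows a rounded-down value as world text and removes itself when done.
; On BeginPlay it records its spawn location and plays a timeline whose vector track offsets the TextRender from that point, then destroys the actor when finished.
; SetDamageText sets the displayed integer, and UpdateRotation sets the text's world rotation.
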(event `self.ReceiveBeginPlay`
  (set `self.StartPos` (`self.K2_GetActorLocation`))
  (bind (_direction `_새_트랙_0`) (`Timeline|DamageText`)
    (:`Update`
      (`SceneComponent.K2_SetWorldLocation` (`self.TextRender`) (+ `_새_트랙_0` (`self.StartPos`)) false false))
    (:`Finished`
      (`self.K2_DestroyActor`))))

(fn `SetDamageText`
  (params (Float :type "Float (double-precision)"))
  (`TextRenderComponent.K2_SetText` (`self.TextRender`) (`KismetTextLibrary.Conv_IntToText` (`KismetMathLibrary.FFloor` Float))))

(fn `UpdateRotation`
  (params (Rotation :type "Rotator Structure"))
  (`SceneComponent.K2_SetWorldRotation` (`self.TextRender`) Rotation false false))

(fn `UserConstructionScript`)